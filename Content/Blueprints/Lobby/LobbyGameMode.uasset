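; Lobby game mode that sets up joining players and can server-travel everyone to the Multiplayer map.
; On authority, PostLogin records the controller, reads server name and player limit from the game instance, and initializes the LobbyPC menu.
; It then respawns the player as a MingerGamesCharacter at a random PlayerStart.
; EveryoneUpdate's player-count broadcast and CanWeStart flag sit behind a never-true count-below-zero check; SwapCharacters and UpdateEveryone are empty.
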(event `Launch Game`
  (`KismetSystemLibrary.ExecuteConsoleCommand` "servertravel /Game/Maps/Multiplayer" null))

(event `self.K2_PostLogin`
  (params (NewPlayer :type "PlayerController Object Reference"))
  ;[1 1 1] Inital Setup, Occurs on first log in post login, handles lobby set up
  (`/Engine/EditorBlueprintResources/ActorMacros.Switch Has Authority`
    (:`Authority`
      (`KismetArrayLibrary.Array_Add` (`self.AllPlayerControllers`) NewPlayer)
      ;;[1 1 1] Can Use this to determine where players spawn
      (bind _outactors (`GameplayStatics.GetAllActorsOfClass` "/Script/Engine.PlayerStart"))
      (set `self.SpawnPoints` _outactors)
      (bind _asour_game_instance (cast `/Game/Blueprints/OurGameInstance` (`GameplayStatics.GetGameInstance`)))
      (set `self.Server Name` (`/Game/Blueprints/OurGameInstance.Server Name` _asour_game_instance))
      (set `self.Max Players` (`/Game/Blueprints/OurGameInstance.MaxPlayers` _asour_game_instance))
      (bind _aslobby_pc (cast `/Game/Blueprints/LobbyPC` NewPlayer))
      (`/Game/Blueprints/LobbyPC.Setup Lobby Menu` _aslobby_pc (`self.Server Name`))
      (`/Game/Blueprints/LobbyPC.Update Lobby Settings` _aslobby_pc (`self.GmMapName`) (`self.GmMapTime`))
      (`self.Respawn Player` NewPlayer))))

(event `Respawn Player`
  (params (`Player Controller` :type "PlayerController Object Reference"))
  (bind _spawnpoints (`self.SpawnPoints`))
  ;[1 1 1] Spawn Player as Base character and tells everyone to update their lobbies
  (`/Engine/EditorBlueprintResources/StandardMacros.IsValid` (`Controller.K2_GetPawn` `Player Controller`)
    (:`Is Valid`
      (`self.K2_DestroyActor`))
    (:`Is Not Valid`
      _))
  (bind _returnvalue (`|SpawnActorFromClass` "/Script/MingerGames.MingerGamesCharacter" (`self.GetTransform` (`|GetArrayItem` _spawnpoints (`KismetMathLibrary.RandomIntegerInRange` 0 (- (`KismetArrayLibrary.Array_Length` _spawnpoints) 1)))) "Undefined" "OverrideRootScale" null null))
  (`Controller.Possess` `Player Controller` _returnvalue)
  (`self.Everyone Update`))

(event `Swap Characters`
  (params (PlayerController :type "PlayerController Object Reference") (ChangedStatus :type Boolean)))

(event `Update Everyone`)

(event `Everyone Update`
  ;[1 1 1] Partially working, updates all lobby information when called
  (bind _output_get (set `self.CurrentPlayers` (`KismetArrayLibrary.Array_Length` (`self.AllPlayerControllers`))))
  (if (< _output_get 0)
    (`KismetArrayLibrary.Array_Clear` (`self.ConnectedPlayers`))
    (for _array_element (`self.AllPlayerControllers`)
      (bind _aslobby_pc (cast `/Game/Blueprints/LobbyPC` _array_element))
      ;;[1 1 1] Hacky work around for player info
      (`/Game/Blueprints/LobbyPC.Update Number of Players` _aslobby_pc (`self.CurrentPlayers`) (`self.Max Players`)))
    (set `self.CanWeStart?` true)))

(fn `UserConstructionScript`)