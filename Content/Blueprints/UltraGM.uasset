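; UltraGM is a game mode that creates local players and spawns first-person characters for them.
; On BeginPlay it caches the game instance, gathers all PlayerStarts and creates one player per NumPlayers.
; SpawnPlayer spawns and possesses a character only when the controller already has a valid pawn.
; GetRandomSpawnPoints supplies the transform, but its random-pick logic is unwired, and DespawnPlayer is an empty stub.
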(event `self.ReceiveBeginPlay`
  (bind _asour_game_instance (cast `/Game/Blueprints/OurGameInstance` (`GameplayStatics.GetGameInstance`))
    (:`then`
      (set `self.GameInstanceRef` _asour_game_instance)
      (bind _outactors (`GameplayStatics.GetAllActorsOfClass` "/Script/Engine.PlayerStart"))
      (set `self.SpawnPoints` _outactors)
      (for _index (range (`/Game/Blueprints/OurGameInstance.NumPlayers` (`self.GameInstanceRef`)))
        (`GameplayStatics.CreatePlayer` _index)))
    (:`CastFailed`
      (`KismetSystemLibrary.PrintString` "Cast to OurGameInstance(ULTRAGM) Failed"))))

(event `Spawn Player`
  (params (Player :type "PlayerController Object Reference"))
  (`/Engine/EditorBlueprintResources/StandardMacros.IsValid` (`Controller.K2_GetPawn` Player)
    (:`Is Valid`
      (bind _returnvalue (`|SpawnActorFromClass` "/Game/FirstPersonCPP/Blueprints/FirstPersonCharacter.FirstPersonCharacter_C" (`self.Get Random Spawn Points`) "Undefined" "OverrideRootScale" null null))
      (`Controller.Possess` Player _returnvalue))
    (:`Is Not Valid`
      (`KismetSystemLibrary.PrintString` "Player Controller is Invalid (ULTRAGM)"))))

(event `Despawn Player`
  (params (`Player Controller` :type "PlayerController Object Reference")))

(fn `UserConstructionScript`)