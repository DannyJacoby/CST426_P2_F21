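; Voxel terrain actor that builds a blocky height-mapped patch of instanced static meshes in its construction script.
; A nested loop over the voxel dimension spaces columns by voxel size and adds one instance each, forming a surface layer.
; ActorLocation derives 2D simplex noise coordinates from the actor's world grid position, cell index and voxel density.
; AddNoise floors the scaled noise into stepped heights for each instance.
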(fn `AddNoise`
  (params (Noise :type "Float (double-precision)") (XTransform :type "Float (double-precision)") (YTransform :type "Float (double-precision)"))
  (`InstancedStaticMeshComponent.AddInstance` (`self.InstancedStaticMesh`) (`KismetMathLibrary.Conv_VectorToTransform` (`KismetMathLibrary.MakeVector` XTransform YTransform (* (`KismetMathLibrary.FFloor` (* 10 Noise)) 100.0)))))

(fn `UserConstructionScript`
  (bind _voxeldimension (`self.VoxelDimension`))
  (bind _returnvalue (`KismetMathLibrary.Conv_IntToDouble` (`self.VoxelSize`)))
  (for _index (range (+ _voxeldimension 1))
    (for _index_2 (range (+ _voxeldimension 1))
      (bind (_x _y) (`self.ActorLocation` _index _index_2))
      (bind _returnvalue_2 (`SimplexNoiseBPLibrary.SimplexNoise2D` _x _y))
      (`self.AddNoise` _returnvalue_2 (* _index _returnvalue) (* _index_2 _returnvalue)))))